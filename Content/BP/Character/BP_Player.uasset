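; BP_Player is a player Blueprint with a 2D scene capture of its own mesh.
; On BeginPlay the SceneCaptureComponent2D is restricted to show only the Mesh, isolating it from the rest of the scene.
; Leftover nodes for toggled yaw rotation and interpolating back to a default rotation are not connected to any event, so they never run.
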(event EventBeginPlay
  (Rendering|SceneCapture|ShowOnlyComponent (Variables|Default|GetSceneCaptureComponent2D) (Variables|Character|GetMesh)))

(event Collision|EventActorBeginOverlap
  (params (OtherActor :type Actor%20Object%20Reference)))

(event EventTick
  (params (DeltaSeconds :type Float%20%28single-precision%29)))

(fn ConstructionScript)