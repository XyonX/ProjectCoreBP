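; Main menu game mode that stages a randomly chosen camera view with a player character on BeginPlay.
; It casts the player pawn to BP_CameraOnlyPawn and picks a random row name from the ViewModeDataTale table variable, then reads that row from DT_ViewMode.
; The row supplies the spawn transform for a BP_Player, plus the camera pawn's teleport transform and FOV.
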(event EventBeginPlay
  (bind _asbp_camera_only_pawn (Utilities|Casting|CastToBP_CameraOnlyPawn (Game|Player|GetPlayerPawn 0)))
  (Variables|Default|SetCameraPawn _asbp_camera_only_pawn)
  (bind _outrownames (DataTable|GetDataTableRowNames (Variables|Default|GetViewModeDataTale)))
  (bind _returnvalue (Utilities|GetDataTableRow "/Game/Data/DT_ViewMode.DT_ViewMode" (.OutItem (Utilities|Array|Random _outrownames)))
    (:then
      (Game|SpawnActorfromClass "/Game/BP/Character/BP_Player.BP_Player_C" (.CharacterWorldLTransform (Utilities|Struct|BreakCameraVewPosData _returnvalue)) "AlwaysSpawn" "MultiplyWithRoot" 0 0)
      (Transformation|SetActorTransform _asbp_camera_only_pawn (.CameraWorldTransform (Utilities|Struct|BreakCameraVewPosData _returnvalue)) false true)
      (Camera|SetFieldOfView (Variables|/Game/BP/Pawn/BP_CameraOnlyPawn.BP_CameraOnlyPawn_C|GetCamera _asbp_camera_only_pawn) (.CameraFOV (Utilities|Struct|BreakCameraVewPosData _returnvalue))))
    (:RowNotFound
      (Development|PrintString "Camera View Set Failed"))))

(fn ConstructionScript)