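; BP_ProceduralGrid is an unfinished world object Blueprint, apparently intended to build a procedural grid mesh.
; On BeginPlay it runs nested Y and X loops sized from map size, scaled by 100, and per-axis vertex density, plus one.
; The loop bodies are empty, the ProceduralMesh section-creation call is never reached, and the construction script is empty, so no geometry is generated.
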(event EventBeginPlay
  (for _index (range 0 (Math|Float|Truncate (+ (* (* (Variables|Default|GetMapSize_Y) 1e+02) (.y (Variables|Default|GetVertexDensity))) 1.0)))
    (for _index_2 (range 0 (Math|Float|Truncate (+ (* (* (Variables|Default|GetMaxSize_X) 1e+02) (.x (Variables|Default|GetVertexDensity))) 1.0)))
      _)))

(event Collision|EventActorBeginOverlap
  (params (OtherActor :type Actor%20Object%20Reference)))

(event EventTick
  (params (DeltaSeconds :type Float%20%28single-precision%29)))

(fn ConstructionScript)