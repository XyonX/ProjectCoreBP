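; BP_AISpawner populates the AI playground with randomly placed BP_TextureAI actors, split at random between friend and enemy.
; On BeginPlay it spawns one BP_FriendAI and one BP_EnemyAI controller, then reads map bounds from BP_GM_AIPlayground.
; SpawnAI places each actor within those bounds at zero height, colors its billboard green or red, and has the matching shared controller possess it, so each controller retains only its latest pawn.
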(event EventBeginPlay
  (Utilities|FlowControl|Sequence
    (:then_0
      (bind _returnvalue (Game|SpawnActorfromClass "/Game/AI/Controller/BP_EnemyAI.BP_EnemyAI_C" (Variables|Default|GetSpawn%20Transform) "AdjustIfPossibleButAlwaysSpawn" "MultiplyWithRoot" 0 0))
      (Variables|Default|SetEnemyAI _returnvalue)
      (bind _returnvalue_2 (Game|SpawnActorfromClass "/Game/AI/Controller/BP_FriendAI.BP_FriendAI_C" (Variables|Default|GetSpawn%20Transform) "AdjustIfPossibleButAlwaysSpawn" "MultiplyWithRoot" 0 0))
      (Variables|Default|SetFriendAI _returnvalue_2))
    (:then_1
      (bind _asbp_gm_aiplayground (Utilities|Casting|CastToBP_GM_AIPlayground (Game|GetGameMode)))
      (bind _output_get (Variables|Default|SetMaxLocation (Variables|/Game/Game/GameMode/BP_GM_AIPlayground.BP_GM_AIPlayground_C|GetMaxLocation _asbp_gm_aiplayground)))
      (Development|PrintString (Utilities|String|ToString(Vector2d) _output_get))
      (Variables|Default|SetMinLocation (Variables|/Game/Game/GameMode/BP_GM_AIPlayground.BP_GM_AIPlayground_C|GetMinLocation _asbp_gm_aiplayground))
      (Variables|Default|SetSurfaceHeight (Variables|/Game/Game/GameMode/BP_GM_AIPlayground.BP_GM_AIPlayground_C|GetSurfaceHeight _asbp_gm_aiplayground))
      (CallFunction|SpawnAI))))

(event Collision|EventActorBeginOverlap
  (params (OtherActor :type Actor%20Object%20Reference)))

(event EventTick
  (params (DeltaSeconds :type Float%20%28single-precision%29)))

(fn ConstructionScript)

(fn SpawnAI
  (bind _minlocation (Variables|Default|GetMinLocation))
  (bind _maxlocation (Variables|Default|GetMaxLocation))
  (for _index (range 0 (Variables|Default|GetNumOfAIS))
    (bind _returnvalue (Game|SpawnActorfromClass "/Game/AI/Pawn/BP_TextureAI.BP_TextureAI_C" (Math|Transform|MakeTransform (Math|Vector|MakeVector (Math|Random|RandomFloatinRange (.x _maxlocation) (.x _minlocation)) (Math|Random|RandomFloatinRange (.y _maxlocation) (.y _minlocation)) 0.0)) "Undefined" "MultiplyWithRoot" 0 0))
    (if (Math|Random|RandomBool)
      (Pawn|Possess (Variables|Default|GetFriendAI) _returnvalue)
      (Rendering|Material|SetMaterial (Variables|/Game/AI/Pawn/BP_TextureAI.BP_TextureAI_C|GetMatBillboard _returnvalue) 0 "/Game/Material/MI_Emmisive_Green.MI_Emmisive_Green")
      (else
        (Pawn|Possess (Variables|Default|GetEnemyAI) _returnvalue)
        (Rendering|Material|SetMaterial (Variables|/Game/AI/Pawn/BP_TextureAI.BP_TextureAI_C|GetMatBillboard _returnvalue) 0 "/Game/Material/MI_Emmisive_RED.MI_Emmisive_RED")))))