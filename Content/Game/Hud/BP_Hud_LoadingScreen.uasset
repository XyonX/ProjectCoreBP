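; HUD Blueprint for the loading screen, which puts the common loading screen widget on screen.
; On BeginPlay it creates WBP_CommonLoadingScreen for the first player controller, stores the reference and adds it to the viewport.
; Disconnected leftover nodes that create a demo widget and add image cards to a loading screen vertical box never run.
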(event EventBeginPlay
  (bind _returnvalue (UserInterface|CreateWidget "/Game/UI/Loading/WBP_CommonLoadingScreen.WBP_CommonLoadingScreen_C" (Game|GetPlayerController 0)))
  (bind _output_get (Variables|Default|SetCommonLoadingScreen _returnvalue))
  (UserInterface|Viewport|AddtoViewport _output_get 0))

(event Collision|EventActorBeginOverlap
  (params (OtherActor :type Actor%20Object%20Reference)))

(event EventTick
  (params (DeltaSeconds :type Float%20%28single-precision%29)))

(fn ConstructionScript)