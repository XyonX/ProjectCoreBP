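; BP_CoreCharacter is a player character Blueprint that handles walking, sprinting, looking, jumping and free look.
; Enhanced Input actions drive movement along the actor's forward and right vectors and rate-scaled look input, while a raw Left Shift key toggles walk speed.
; Holding IA_EyeRotation decouples body yaw from the controller; releasing it snaps the view back to actor yaw with level pitch and restores coupling.
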(event Input|EnhancedActionEvents|EnhancedInputActionIA_Movement
  (params (ActionValue :type Vector%202D%20Structure) (ElapsedSeconds :type Float%20%28double-precision%29) (TriggeredSeconds :type Float%20%28double-precision%29) (InputAction :type Input%20Action%20Object%20Reference :default "/Game/Input/Actions/IA_Movement.IA_Movement"))
  (:Triggered
    (Pawn|Input|AddMovementInput (Transformation|GetActorForwardVector) (.x ActionValue) false)
    (Pawn|Input|AddMovementInput (Transformation|GetActorRightVector) (.y ActionValue) false)))

(event Input|EnhancedActionEvents|EnhancedInputActionIA_Looking
  (params (ActionValue :type Vector%202D%20Structure) (ElapsedSeconds :type Float%20%28double-precision%29) (TriggeredSeconds :type Float%20%28double-precision%29) (InputAction :type Input%20Action%20Object%20Reference :default "/Game/Input/Actions/IA_Looking.IA_Looking"))
  (:Triggered
    (Pawn|Input|AddControllerYawInput (* (.x ActionValue) (Variables|Default|GetTurnRate)))
    (Pawn|Input|AddControllerPitchInput (* (.y ActionValue) (Variables|Default|GetLookUpRate)))))

(event Input|EnhancedActionEvents|EnhancedInputActionIA_Jump
  (params (ActionValue :type Boolean) (ElapsedSeconds :type Float%20%28double-precision%29) (TriggeredSeconds :type Float%20%28double-precision%29) (InputAction :type Input%20Action%20Object%20Reference :default "/Game/Input/Actions/IA_Jump.IA_Jump"))
  (:Triggered
    (Character|Jump)))

(event Input|EnhancedActionEvents|EnhancedInputActionIA_EyeRotation
  (params (ActionValue :type Boolean) (ElapsedSeconds :type Float%20%28double-precision%29) (TriggeredSeconds :type Float%20%28double-precision%29) (InputAction :type Input%20Action%20Object%20Reference :default "/Game/Input/Actions/IA_EyeRotation.IA_EyeRotation"))
  (:Triggered
    (Variables|Default|SetbUseControllerRotationYaw false))
  (:Completed
    (Pawn|SetControlRotation (Game|GetPlayerController 0) (Math|Rotator|MakeRotator 0.0 0.0 (.Yaw (Math|Rotator|BreakRotator (Transformation|GetActorRotation)))))
    (Variables|Default|SetbUseControllerRotationYaw true)))

(event EventBeginPlay)

(event Collision|EventActorBeginOverlap
  (params (OtherActor :type Actor%20Object%20Reference)))

(event EventTick
  (params (DeltaSeconds :type Float%20%28single-precision%29)))

(event Input|KeyboardEvents|LeftShift
  (params (Key :type Key%20Structure :default "None"))
  (bind _charactermovement (Variables|Character|GetCharacterMovement))
  (:Pressed
    (Variables|/Script/Engine.CharacterMovementComponent|SetMaxWalkSpeed _charactermovement 4e+02))
  (:Released
    (Variables|/Script/Engine.CharacterMovementComponent|SetMaxWalkSpeed _charactermovement 2e+02)))

(fn ConstructionScript)